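; LookTarget is a component that lets its owning actor react to being looked at by the player, tracking hover state and highlighting it.
; On BeginPlay it binds to the look start and end events of BP_ThirdPersonCharacter, responding only when the target is its owner.
; Hover toggles custom depth and stencil on the owner's static meshes for an outline, with only enabling gated by ShouldRenderOutline.
; GetIsHovered exposes the state; hover stop also prints a leftover debug string.
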(event Custom|EventLookStart_Event
  (params (LookTarget :type Actor%20Object%20Reference))
  (if (== LookTarget (Components|GetOwner))
    (Variables|Default|SetIsHovered true)
    (CallFunction|HandleHoverStart)))

(event Custom|EventLookEnd_Event
  (params (LookTarget :type Actor%20Object%20Reference))
  (if (== LookTarget (Components|GetOwner))
    (Variables|Default|SetIsHovered false)
    (CallFunction|HandleHoverStop)))

(event EventBeginPlay
  (bind _asbp_third_person_character (Utilities|Casting|CastToBP_ThirdPersonCharacter (Game|GetPlayerCharacter 0))
    (:then
      (EventDispatchers|BindEventtoEventLookStart _asbp_third_person_character (delegate Custom|EventLookStart_Event))
      (EventDispatchers|BindEventtoEventLookEnd _asbp_third_person_character (delegate Custom|EventLookEnd_Event)))
    (:CastFailed
      (Development|PrintString (Utilities|GetDisplayName _asbp_third_person_character)))))

(fn HandleHoverStart
  (if (Variables|Default|GetShouldRenderOutline)
    (for _array_element (Actor|GetComponentsByClass (Components|GetOwner) "/Script/Engine.StaticMeshComponent")
      (Rendering|SetRenderCustomDepth _array_element true)
      (Rendering|SetCustomDepthStencilValue _array_element 1))))

(fn HandleHoverStop
  (Development|PrintString "Bitch")
  (for _array_element (Actor|GetComponentsByClass (Components|GetOwner) "/Script/Engine.StaticMeshComponent")
    (Rendering|SetRenderCustomDepth _array_element false)
    (Rendering|SetCustomDepthStencilValue _array_element 0)))

(fn GetIsHovered
  (return (Variables|Default|GetIsHovered)))